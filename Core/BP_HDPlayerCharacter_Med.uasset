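; Player character adding a medic revive system, driven by the MedicalState on its player controller.
; A first death leaves the player Wounded with a revive spawner; dying while Revived means Dead.
; Revived spawns regain their kit at low health and go prone, returning to Normal after a timer or full heal.
; Inventory checks for a medic box set the Medic flag and toggle controller UI, through helpers whose names are inverted.
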(event Custom|ServerEquipKit
  (bind _medcontroller (Variables|Default|GetMedController))
  ;[1 1 1] Picks up nearby kit on Revive
  ;
  ; Sets a timer that sets Medical State to Normal after elapsed time.
  (Networking|SwitchHasAuthority
    (:Authority
      (if (Utilities|Enum|Equal(Enum) (Variables|/MedicalTest/Core/BP_HDPlayerController_MedTest.BP_HDPlayerController_MedTest_C|GetMedicalState _medcontroller) "NewEnumerator1")
        (Class|HDPlayerCharacter|OnPickupKit (Variables|/MedicalTest/Core/BP_HDPlayerController_MedTest.BP_HDPlayerController_MedTest_C|GetPickupItem _medcontroller))
        (Variables|Default|SetHealth 2e+01)
        (bind _returnvalue (Utilities|Time|SetTimerbyEvent (delegate Custom|InstaDeathCounter) (Variables|Default|GetTimeToClearInstaDeath)))
        (Variables|Default|SetInstaDeathHandle _returnvalue)))))

(event Custom|ClientCheckIfMedic
  ;[1 1 1] CheckIfMedic (Fairly Inefficient and Sketchy Solution)
  ;;[1 0.6858 0.02494] CheckIfMedicOnKitPickup
  ;;
  ;; On Client to deal make working with UI easier
  (CallFunction|CheckifMedic))

(event Custom|ClearRevivedOnFullHeal
  (params (Character :type DF%20Base%20Character%20Object%20Reference) (NewHealthTotal :type Float%20%28single-precision%29) (PrevHealthTotal :type Float%20%28single-precision%29))
  ;[1 1 1] Pickup Nearby Kit and Prone if Revived then Check if Medic
  ;
  ; Otherwise just Check if Medic if Spawned Normally
  ;;[1 0.3193 0] If Health Reaches Full After Being Recently Player is Revivable On Death
  (if (and (== NewHealthTotal 1e+02) (Utilities|Enum|Equal(Enum) (Variables|/MedicalTest/Core/BP_HDPlayerController_MedTest.BP_HDPlayerController_MedTest_C|GetMedicalState (Variables|Default|GetMedController)) "NewEnumerator1"))
    (Variables|/MedicalTest/Core/BP_HDPlayerController_MedTest.BP_HDPlayerController_MedTest_C|SetMedicalState (Variables|Default|GetMedController) "NewEnumerator0")
    (CallFunction|ClearTimer (Variables|Default|GetInstaDeathHandle))))

(event Custom|InstaDeathCounter
  ;[1 1 1] Picks up nearby kit on Revive
  ;
  ; Sets a timer that sets Medical State to Normal after elapsed time.
  (Variables|/MedicalTest/Core/BP_HDPlayerController_MedTest.BP_HDPlayerController_MedTest_C|SetMedicalState (Variables|Default|GetMedController) "NewEnumerator0")
  (Utilities|Time|ClearandInvalidateTimerbyHandle (Variables|Default|GetInstaDeathHandle)))

(event Custom|CheckIfMedic
  ;[1 1 1] CheckIfMedic (Fairly Inefficient and Sketchy Solution)
  ;;[1 0 0.7758] Checks if Medic and displays or hides medic UI (depending on if medical kit is in inventory)
  ;;
  ;; CanMedicCheck is there to prevent CheckIfMedicOnKitPickup from firing on spawn as it is triggered twice for some reason and triggers before some begin play variables are initialized
  (if (and (Class|DFBlueprintFunctions|IsLocallyPlayerControlled) (Variables|Default|GetCanMedicCheck))
    (Variables|Default|SetIsMedicAssigned false)
    (bind _array_element (Utilities|Array|ForEachLoopwithBreak (Variables|/Script/DonkehFramework.DFInventoryComponent|GetItems (Variables|Default|GetInventory)) :!label _label)
      (:LoopBody
        (if (Utilities|ClassIsChildOf (Utilities|GetClass _array_element) "/HDCore/Core/Items/BP_HDWeap_MedicBoxBase.BP_HDWeap_MedicBoxBase_C")
          (Variables|Default|SetIsMedicAssigned true)
          (CallFunction|ServerSetMedic true)
          (Development|PrintString "MedicPicked" true true "(R=1.000000,G=0.000000,B=0.095176,A=1.000000)")
          (Utilities|DisableMedicUI)
          (goto _label Break)))
      (:Completed
        (if (not (Variables|Default|GetIsMedicAssigned))
          (Development|PrintString "MedicNotPicked" true true "(R=1.000000,G=0.000000,B=0.095176,A=1.000000)")
          (CallFunction|ServerSetMedic false)
          (Utilities|EnableMedicUI))))))

(event Custom|ServerSetMedic
  (params (Medic :type Boolean))
  ;[1 1 1] CheckIfMedic (Fairly Inefficient and Sketchy Solution)
  ;;[1 0 0.7758] Checks if Medic and displays or hides medic UI (depending on if medical kit is in inventory)
  ;;
  ;; CanMedicCheck is there to prevent CheckIfMedicOnKitPickup from firing on spawn as it is triggered twice for some reason and triggers before some begin play variables are initialized
  (Variables|Default|SetMedic Medic))

(event EventOnDeath
  (params (KillingDamage :type Float%20%28single-precision%29) (DamageEvent :type Damage%20Event%20Structure%20%28by%20ref%29) (InstigatingPawn :type Pawn%20Object%20Reference) (DamageCauser :type Actor%20Object%20Reference))
  (bind _self self)
  (bind _medcontroller (Variables|Default|GetMedController))
  ;[1 1 1] Clears Timers and Checks whether to set to Wounded or Dead.
  ;
  ; If wounded spawns Revive Actor
  (|CallParentFunction KillingDamage DamageEvent InstigatingPawn DamageCauser)
  (CallFunction|ClearTimer (Variables|Default|GetMedicTimer))
  (CallFunction|ClearTimer (Variables|Default|GetInstaDeathHandle))
  (Networking|SwitchHasAuthority
    (:Authority
      (switch Utilities|FlowControl|Switch|SwitchonMedicalStateEnum (Variables|/MedicalTest/Core/BP_HDPlayerController_MedTest.BP_HDPlayerController_MedTest_C|GetMedicalState _medcontroller)
        (:NewEnumerator0
          (Variables|/MedicalTest/Core/BP_HDPlayerController_MedTest.BP_HDPlayerController_MedTest_C|SetMedicalState _medcontroller "NewEnumerator2")
          (Default|AddReviveSpawner (Variables|Default|GetMedController) (Transformation|GetActorTransform _self) (Variables|Default|GetTeamNum _self)))
        (:NewEnumerator1
          (Variables|/MedicalTest/Core/BP_HDPlayerController_MedTest.BP_HDPlayerController_MedTest_C|SetMedicalState _medcontroller "NewEnumerator3"))))))

(event EventBeginPlay
  ;[1 1 1] Pickup Nearby Kit and Prone if Revived then Check if Medic
  ;
  ; Otherwise just Check if Medic if Spawned Normally
  (|CallParentFunction)
  (Utilities|FlowControl|Delay 0.1)
  (bind _asbp_hdplayer_controller_med_test (Utilities|Casting|CastToBP_HDPlayerController_MedTest (Pawn|GetController)))
  (Variables|Default|SetMedController _asbp_hdplayer_controller_med_test)
  (EventDispatchers|AssignOnHealthChanged (delegate Custom|ClearRevivedOnFullHeal))
  (if (Utilities|Enum|Equal(Enum) (Variables|/MedicalTest/Core/BP_HDPlayerController_MedTest.BP_HDPlayerController_MedTest_C|GetMedicalState (Variables|Default|GetMedController)) "NewEnumerator1")
    (CallFunction|ServerEquipKit)
    (Class|DFBaseCharacter|ProneToggle)
    (Variables|Default|SetCanMedicCheck true)
    (CallFunction|CheckifMedic)
    (else
      (Variables|Default|SetCanMedicCheck true)
      (CallFunction|CheckifMedic))))

(event EventCurrentLoadout
  ;[1 1 1] CheckIfMedic (Fairly Inefficient and Sketchy Solution)
  ;;[1 0.6858 0.02494] CheckIfMedicOnKitPickup
  ;;
  ;; On Client to deal make working with UI easier
  (|CallParentFunction)
  (CallFunction|ClientCheckifMedic))

(fn ConstructionScript
  (|CallParentFunction))

(fn ClearTimer
  (params (Handle :type Timer%20Handle%20Structure))
  (if (Utilities|Time|IsTimerActivebyHandle Handle)
    (Utilities|Time|ClearandInvalidateTimerbyHandle Handle)))

(fn OnRepMedic
  (bind _medcontroller (Variables|Default|GetMedController))
  (bind _medcontroller_2 (Variables|Default|GetMedController))
  (if (Class|DFBlueprintFunctions|IsLocallyPlayerControlled)
    (if (Variables|Default|GetMedic)
      (Utilities|IsValid _medcontroller_2
        (:Is%20Valid
          (Default|EnableMedicUI _medcontroller_2))
        (:Is%20Not%20Valid
          _))
      (else
        (Utilities|IsValid _medcontroller
          (:Is%20Valid
            (Default|DisableMedicUI _medcontroller))
          (:Is%20Not%20Valid
            _))))
    (Development|PrintString "ONREP" true true "(R=1.000000,G=0.000000,B=0.890917,A=1.000000)")))
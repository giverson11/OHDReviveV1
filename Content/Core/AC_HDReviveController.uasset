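; Player controller component that runs the medic revive system through Normal, Wounded, Revived and Dead medical states.
; MedicalState's OnRep drives wounded and death screens, revive actor cleanup, and respawning revived players at their stored death transform with an unarmed loadout.
; Medics line-trace for a revive spawner, with a retriggerable delay and gate implementing hold-to-revive before calling ServerRevive.
; A looping timer refreshes team-based visibility of revive markers while medic UI is enabled.
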(event Custom|AddReviveSpawner
  (params (DeathTransform :type Transform) (TeamNum :type Byte))
  ;[1 1 1] Spawn the Revive Actor and Revive Spawn Actor
  (bind _revivetransform (Utilities|CreateReviveSpawner DeathTransform TeamNum)
    (:Exit
      (Variables|Default|SetReviveTransform _revivetransform))))

(event Custom|RevivePlayer
  ;[1 1 1] Helpers
  (Variables|Default|SetMedicalState "NewEnumerator1"))

(event Custom|ServerRevive
  (params (Revive :type BP%20HD%20Revive%20Spawner%20Object%20Reference) (PlayerReviveComponent :type AC%20HD%20Revive%20Character%20Object%20Reference) (Team :type Byte))
  ;[1 1 1] Trace For Revive Actor
  ;
  ; Check USE Is Held For ReviveHoldTIme
  ;
  ; and Initiate Revive
  (Default|Revive Revive PlayerReviveComponent Team))

(event Custom|InitiateRevive
  ;[1 1 1] Trace For Revive Actor
  ;
  ; Check USE Is Held For ReviveHoldTIme
  ;
  ; and Initiate Revive
  (if (Variables|/MedicalTest/Core/AC_HDReviveCharacter.AC_HDReviveCharacter_C|GetMedic (Variables|Default|GetPlayerReviveComp))
    (bind _hdrevive_spawner (Utilities|TraceforReviveActor)
      (:Exit
        (Default|StartFillingProgressBar _hdrevive_spawner)
        (CallFunction|OnHold)
        (Utilities|FlowControl|Gate true) ; enters at Open
      ))
    (else
      (Development|PrintString "NotMedic" true true "(R=1.000000,G=0.000000,B=0.019754,A=1.000000)"))))

(event Custom|OnHold
  ;[1 1 1] Trace For Revive Actor
  ;
  ; Check USE Is Held For ReviveHoldTIme
  ;
  ; and Initiate Revive
  (Utilities|FlowControl|RetriggerableDelay (Variables|Default|GetReviveHoldTime))
  (Utilities|FlowControl|Gate true
    (:Exit
      (CallFunction|ServerRevive (stale Custom|InitiateRevive _hdrevive_spawner) (Variables|Default|GetPlayerReviveComp) (Class|DFBlueprintFunctions|GetTeamNum (Variables|/MedicalTest/Core/AC_HDReviveCharacter.AC_HDReviveCharacter_C|GetPlayerChar (Variables|Default|GetPlayerReviveComp)))))))

(event Custom|OnWounded
  ;[0.9583 1 0.9167] OnRep Medical States: Triggers when Player's medical States changes (Normal, Revivable, Wounded, Death)
  ;;[1 0.2633 0] OnWounded (Player is incapaciatated but Revivable)
  (Development|PrintString "Wounded" true true "(R=1.000000,G=0.402985,B=0.000000,A=1.000000)")
  (Networking|CanExecuteCosmeticEvents
    (:True
      (CallFunction|WoundedScreenToggle true))))

(event Custom|OnRevived
  ;[0.9583 1 0.9167] OnRep Medical States: Triggers when Player's medical States changes (Normal, Revivable, Wounded, Death)
  ;;[1 0.9253 0] OnRevived(Player is Alive but will become Dead (unrevivable) on Death)
  (Utilities|OwnerHasAuthority
    (:Authority
      (Development|PrintString "Revived" true true "(R=1.000000,G=0.809269,B=0.000000,A=1.000000)")
      (CallFunction|GetReviveKit)
      (Class|GameModeBase|RestartPlayeratTransform (Game|GetGameMode) (Variables|Default|GetController) (Variables|Default|GetReviveTransform))
      (CallFunction|DestroyRevive))
    (:Remote
      _))
  (Networking|CanExecuteCosmeticEvents
    (:True
      (CallFunction|WoundedScreenToggle false))))

(event Custom|EnableMedicUI
  ;[1 1 1] Handles Revive Icon UI
  (if (Utilities|Time|IsValidTimerHandle (Variables|Default|GetMedicHandle))
    (Utilities|Time|UnpauseTimerbyHandle (Variables|Default|GetMedicHandle))
    (else
      (bind _returnvalue (Utilities|Time|SetTimerbyEvent (delegate Custom|MedicTimer) 0.3 true))
      (Variables|Default|SetMedicHandle _returnvalue))))

(event Custom|DestroyRevive
  ;[1 1 1] DestroyReviveActor/ReviveStart
  (Utilities|OwnerHasAuthority
    (:Authority
      (Utilities|IsValid (Variables|Default|GetRevive)
        (:Is%20Valid
          (Actor|DestroyActor (Variables|Default|GetRevive))
          (Variables|Default|SetRevive 0))
        (:Is%20Not%20Valid
          (Development|PrintString "DestroyingInvalidRevive"))))))

(event Custom|DisableMedicUI
  ;[1 1 1] Handles Revive Icon UI
  (if (Utilities|Time|IsValidTimerHandle (Variables|Default|GetMedicHandle))
    (Utilities|Time|PauseTimerbyHandle (Variables|Default|GetMedicHandle)))
  (for _array_element (Variables|Default|GetReviveSpawners)
    (Default|HideReviveSpawner _array_element)))

(event Custom|MedicTimer
  ;[1 1 1] Handles Revive Icon UI
  (for _array_element (Variables|Default|GetReviveSpawners)
    (Default|CheckTeamforVisibility _array_element (Variables|/MedicalTest/Core/AC_HDReviveCharacter.AC_HDReviveCharacter_C|GetPlayerChar (Variables|Default|GetPlayerReviveComp)))))

(event Custom|OnDead
  ;[0.9583 1 0.9167] OnRep Medical States: Triggers when Player's medical States changes (Normal, Revivable, Wounded, Death)
  ;;[1 0 0.02628] OnDead (Player is incapacitated but unable to be revived "DeadDead')
  (CallFunction|DestroyRevive)
  (Networking|CanExecuteCosmeticEvents
    (:True
      (Default|DeathScreenToggle (Variables|Default|GetController) true)
      (CallFunction|WoundedScreenToggle false))))

(event Custom|OnNormal
  ;[0.9583 1 0.9167] OnRep Medical States: Triggers when Player's medical States changes (Normal, Revivable, Wounded, Death)
  ;;[0.01576 1 0] OnNormal(Player is Alive and Will Become Wounded On Death)
  (Development|PrintString "Normal" true true "(R=0.086353,G=1.000000,B=0.040309,A=1.000000)")
  (Networking|CanExecuteCosmeticEvents
    (:True
      (Default|DeathScreenToggle (Variables|Default|GetController) false)
      (CallFunction|WoundedScreenToggle false))))

(event Custom|KillPlayer
  ;[1 1 1] Helpers
  (Utilities|OwnerHasAuthority
    (:Authority
      (Variables|Default|SetMedicalState "NewEnumerator3"))
    (:Remote
      (CallFunction|ServerKillPlayer))))

(event Custom|ServerKillPlayer
  ;[1 1 1] Helpers
  (Variables|Default|SetMedicalState "NewEnumerator3"))

(event Custom|ReleaseCancel
  ;[1 1 1] Trace For Revive Actor
  ;
  ; Check USE Is Held For ReviveHoldTIme
  ;
  ; and Initiate Revive
  (Utilities|FlowControl|Gate true) ; enters at Close
)

(event Custom|OnUnpossess
  (params (Pawn :type Pawn%20Object%20Reference))
  ;[1 1 1] Handles Revive Icon UI
  (Networking|CanExecuteCosmeticEvents
    (:True
      (CallFunction|DisableMedicUI))))

(event Custom|PlayerTeamNumberUpdated
  (params (LastTeamNum :type Byte) (NewTeamNum :type Byte))
  ;[1 1 1] SetToDeadOnTeamChange
  (if (Utilities|Enum|NotEqual(Enum) (Variables|Default|GetMedicalState) "NewEnumerator3")
    (Variables|Default|SetMedicalState "NewEnumerator3")))

(event Custom|OnPossess
  (params (NewPawn :type Pawn%20Object%20Reference))
  (bind _returnvalue (Actor|GetComponentbyClass NewPawn "/MedicalTest/Core/AC_HDReviveCharacter.AC_HDReviveCharacter_C"))
  ;[1 1 1] ResetMedicalStateOnSpawn
  (Utilities|IsValid _returnvalue
    (:Is%20Valid
      (Variables|Default|SetPlayerReviveComp _returnvalue)
      (if (Utilities|Enum|Equal(Enum) (Variables|Default|GetMedicalState) "NewEnumerator2")
        (CallFunction|DestroyRevive)
        (Variables|Default|SetMedicalState "NewEnumerator0" :!label _label)
        (elif (Utilities|Enum|Equal(Enum) (Variables|Default|GetMedicalState) "NewEnumerator3")
          (goto _label))))
    (:Is%20Not%20Valid
      (Development|PrintString "ComponentIsNotValid" true true "(R=0.000000,G=0.660000,B=1.000000,A=1.000000)" 7.0))))

(event EventTick
  (params (DeltaSeconds :type Float%20%28single-precision%29)))

(event EventBeginPlay
  (bind _asbp_hdplayer_controller_base (Utilities|Casting|CastToBP_HDPlayerControllerBase (Components|GetOwner))
    (:then
      (Variables|Default|SetController _asbp_hdplayer_controller_base)
      (Development|PrintString "ReviveControllerStarting" true true "(R=1.000000,G=0.970537,B=0.992634,A=1.000000)")
      (CallFunction|LoadWoundedScreen)
      (EventDispatchers|BindEventtoOnPossessPawn (Variables|Default|GetController) (EventDispatchers|CreateEvent :!event Custom|OnPossess))
      (EventDispatchers|BindEventtoOnUnpossessPawn (Variables|Default|GetController) (EventDispatchers|CreateEvent :!event Custom|OnUnpossess))
      (EventDispatchers|BindEventtoOnPlayerTeamNumUpdated (Variables|Default|GetController) (EventDispatchers|CreateEvent :!event Custom|PlayerTeamNumberUpdated)))
    (:CastFailed
      (Components|Activation|Deactivate)
      (Development|PrintString "ControllerCastFailed" true true "(R=1.000000,G=0.983531,B=0.962442,A=1.000000)"))))

(fn OnRepMedicalState
  (Development|PrintString "OnRep")
  (switch Utilities|FlowControl|Switch|SwitchonMedicalStateEnum (Variables|Default|GetMedicalState)
    (:NewEnumerator0
      (CallFunction|OnNormal))
    (:NewEnumerator1
      (CallFunction|OnRevived))
    (:NewEnumerator2
      (CallFunction|OnWounded))
    (:NewEnumerator3
      (CallFunction|OnDead))))

(fn WoundedScreenToggle
  (params (Show :type Boolean))
  (bind _woundedwidget (Variables|Default|GetWoundedWidget))
  (bind _returnvalue (UserInterface|Viewport|IsinViewport _woundedwidget))
  (Utilities|IsValid _woundedwidget
    (:Is%20Valid
      (if Show
        (if (not _returnvalue)
          (UserInterface|Viewport|AddtoPlayerScreen (Variables|Default|GetWoundedWidget))
          (bind _output_get (LocalVariables|SetbWoundedScreenShown Show :!label _label))
          (if _output_get
            (Default|HideHUD (Variables|Default|GetController))
            (else
              (Default|ShowHUD (Variables|Default|GetController)))))
        (elif _returnvalue
          (Widget|RemovefromParent (Variables|Default|GetWoundedWidget))
          (goto _label))))))

(fn LoadWoundedScreen
  (Utilities|IsValid (Variables|Default|GetWoundedWidget)
    (:Is%20Not%20Valid
      (bind _returnvalue (UserInterface|CreateWidget "/MedicalTest/Core/UI/Revive/WBP_WoundedScreenRevive.WBP_WoundedScreenRevive_C" (Variables|Default|GetController)))
      (Variables|Default|SetWoundedWidget _returnvalue))))

(fn GetReviveKit
  (bind _revivetransform (Variables|Default|GetReviveTransform))
  (bind _outhits (Collision|MultiSphereTraceByChannel (.location _revivetransform) (.location _revivetransform) 2e+02 "TraceTypeQuery1" false 0 "None"))
  (bind _array_element (Utilities|Array|ForEachLoopwithBreak _outhits :!label _label)
    (:LoopBody
      (if (Utilities|ClassIsChildOf (Utilities|GetClass (|GetHitActor_2_2_2_2 _array_element)) "/HDCore/Core/BP_HDKitPickupBase.BP_HDKitPickupBase_C")
        (bind _asbp_hdkit_pickup_base (Utilities|Casting|CastToBP_HDKitPickupBase (|GetHitActor_2_2_2_2 _array_element)))
        (Variables|Default|SetPickupItem _asbp_hdkit_pickup_base)
        (if (== (Utilities|GetClass (|GetHitActor_2_2_2_2 _array_element)) (Variables|/Script/HDMain.HDKit|GetKitDropPrefabClass (Variables|/Script/HDMain.HDPlayerState|GetSpawnLoadout (Default|GetHDPlayerState (Variables|Default|GetController)))))
          (goto _label Break))))
    (:Completed
      (Variables|/Script/HDMain.HDPlayerComponent|SetStartLoadout (Variables|/Script/HDMain.HDPlayerController|GetPlayerComponent (Variables|Default|GetController)) "/MedicalTest/Core/Kits/HDKit_Unarmed.HDKit_Unarmed"))))
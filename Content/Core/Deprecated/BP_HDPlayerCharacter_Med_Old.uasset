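; Deprecated player character for a medic and revive system, with live hooks delegating to a ReviveComponent.
; Possession initializes the component, and loadout updates trigger its server-side medic check.
; Older in-character logic remains for inventory-based medic detection with UI toggling, and revived kit re-equip at low health with a timer clearing instant-death risk.
; The BeginPlay revive setup and OnDeath wounded/dead branching are disconnected.
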(event Custom|ServerEquipKit
  ;[1 1 1] Picks up nearby kit on Revive
  ;
  ; Sets a timer that sets Medical State to Normal after elapsed time.
  (Class|DFBaseCharacter|ProneToggle)
  (CallFunction|EquipKit))

(event Custom|ClientCheckIfMedic
  ;[1 1 1] CheckIfMedic (Fairly Inefficient and Sketchy Solution)
  ;;[1 0.6858 0.02494] CheckIfMedicOnKitPickup
  (CallFunction|CheckifMedic))

(event Custom|EquipKit
  (bind _returnvalue (Pawn|GetController))
  (bind _asbp_hdplayer_controller_med_test (Utilities|Casting|CastToBP_HDPlayerController_MedTest _returnvalue))
  (bind _pickupitem (Variables|/MedicalTest/Core/BP_HDPlayerController_MedTest.BP_HDPlayerController_MedTest_C|GetPickupItem _asbp_hdplayer_controller_med_test))
  ;[1 1 1] Picks up nearby kit on Revive
  ;
  ; Sets a timer that sets Medical State to Normal after elapsed time.
  (Development|PrintString "Equipping" true true "(R=0.133759,G=0.000000,B=1.000000,A=1.000000)" 5.0)
  (if (Utilities|Enum|Equal(Enum) (Variables|/MedicalTest/Core/BP_HDPlayerController_MedTest.BP_HDPlayerController_MedTest_C|GetMedicalState _asbp_hdplayer_controller_med_test) "NewEnumerator1")
    (Utilities|IsValid _pickupitem
      (:Is%20Valid
        (Class|HDPlayerCharacter|OnPickupKit _pickupitem))
      (:Is%20Not%20Valid
        _))
    (Variables|Default|SetHealth 2e+01)
    (bind _returnvalue_2 (Utilities|Time|SetTimerbyEvent (delegate Custom|InstaDeathCounter) (Variables|Default|GetTimeToClearInstaDeath)))
    (Variables|Default|SetInstaDeathHandle _returnvalue_2)))

(event Custom|ClearRevivedOnFullHeal
  (params (Character :type DF%20Base%20Character%20Object%20Reference) (NewHealthTotal :type Float%20%28single-precision%29) (PrevHealthTotal :type Float%20%28single-precision%29))
  ;[1 1 1] Pickup Nearby Kit and Prone if Revived then Check if Medic
  ;
  ; Otherwise just Check if Medic if Spawned Normally
  ;;[1 0.3193 0] If Health Reaches Full After Being Recently Player is Revivable On Death
  (if (and (== NewHealthTotal 1e+02) (Utilities|Enum|Equal(Enum) (Variables|/MedicalTest/Core/Deprecated/BP_HDPlayerController_MedTestOld.BP_HDPlayerController_MedTestOld_C|GetMedicalState (Variables|Default|GetMedController)) "NewEnumerator1"))
    (Variables|/MedicalTest/Core/Deprecated/BP_HDPlayerController_MedTestOld.BP_HDPlayerController_MedTestOld_C|SetMedicalState (Variables|Default|GetMedController) "NewEnumerator0")
    (CallFunction|ClearTimer (Variables|Default|GetInstaDeathHandle))))

(event Custom|InstaDeathCounter
  ;[1 1 1] Picks up nearby kit on Revive
  ;
  ; Sets a timer that sets Medical State to Normal after elapsed time.
  (Variables|/MedicalTest/Core/Deprecated/BP_HDPlayerController_MedTestOld.BP_HDPlayerController_MedTestOld_C|SetMedicalState (Variables|Default|GetMedController) "NewEnumerator0")
  (Utilities|Time|ClearandInvalidateTimerbyHandle (Variables|Default|GetInstaDeathHandle)))

(event Custom|SetMedic
  (params (Medic :type Boolean))
  ;[1 1 1] CheckIfMedic (Fairly Inefficient and Sketchy Solution)
  ;;[1 0 0.7758] Checks if Medic and displays or hides medic UI (depending on if medical kit is in inventory)
  ;;
  ;; CanMedicCheck is there to prevent CheckIfMedicOnKitPickup from firing on spawn as it is triggered twice for some reason and triggers before some begin play variables are initialized
  (Variables|Default|SetMedic Medic))

(event Custom|CheckIfMedic
  ;[1 1 1] CheckIfMedic (Fairly Inefficient and Sketchy Solution)
  ;;[1 0 0.7758] Checks if Medic and displays or hides medic UI (depending on if medical kit is in inventory)
  ;;
  ;; CanMedicCheck is there to prevent CheckIfMedicOnKitPickup from firing on spawn as it is triggered twice for some reason and triggers before some begin play variables are initialized
  (if (and (Class|DFBlueprintFunctions|IsLocallyPlayerControlled) (Variables|Default|GetCanMedicCheck))
    (Variables|Default|SetIsMedicAssigned false)
    (bind _array_element (Utilities|Array|ForEachLoopwithBreak (Variables|/Script/DonkehFramework.DFInventoryComponent|GetItems (Variables|Default|GetInventory)) :!label _label)
      (:LoopBody
        (if (Utilities|MedboxCheck _array_element)
          (Variables|Default|SetIsMedicAssigned true)
          (Networking|SwitchHasAuthority
            (:Authority
              (CallFunction|SetMedic true))
            (:Remote
              (CallFunction|ServerSetMedic true)))
          (Development|PrintString "MedicPicked" true true "(R=1.000000,G=0.000000,B=0.095176,A=1.000000)")
          (Utilities|EnableMedicUI)
          (goto _label Break)))
      (:Completed
        (if (not (Variables|Default|GetIsMedicAssigned))
          (Development|PrintString "MedicNotPicked" true true "(R=1.000000,G=0.000000,B=0.095176,A=1.000000)")
          (Networking|SwitchHasAuthority
            (:Authority
              (CallFunction|SetMedic false))
            (:Remote
              (CallFunction|ServerSetMedic false)))
          (Utilities|DisableMedicUI))))))

(event Custom|ServerSetMedic
  (params (Medic :type Boolean))
  ;[1 1 1] CheckIfMedic (Fairly Inefficient and Sketchy Solution)
  ;;[1 0 0.7758] Checks if Medic and displays or hides medic UI (depending on if medical kit is in inventory)
  ;;
  ;; CanMedicCheck is there to prevent CheckIfMedicOnKitPickup from firing on spawn as it is triggered twice for some reason and triggers before some begin play variables are initialized
  (CallFunction|SetMedic Medic))

(event EventOnDeath
  (params (KillingDamage :type Float%20%28single-precision%29) (DamageEvent :type Damage%20Event%20Structure%20%28by%20ref%29) (InstigatingPawn :type Pawn%20Object%20Reference) (DamageCauser :type Actor%20Object%20Reference))
  ;[1 1 1] Clears Timers and Checks whether to set to Wounded or Dead.
  ;
  ; If wounded spawns Revive Actor
  (|CallParentFunction KillingDamage DamageEvent InstigatingPawn DamageCauser))

(event EventBeginPlay
  ;[1 1 1] Pickup Nearby Kit and Prone if Revived then Check if Medic
  ;
  ; Otherwise just Check if Medic if Spawned Normally
  (|CallParentFunction))

(event EventCurrentLoadout
  ;[1 1 1] CheckIfMedic (Fairly Inefficient and Sketchy Solution)
  ;;[1 0.6858 0.02494] CheckIfMedicOnKitPickup
  (|CallParentFunction)
  (Networking|SwitchHasAuthority
    (:Authority
      (Default|CheckifMedic (Variables|Default|GetReviveComponent)))))

(event EventTick
  (params (DeltaSeconds :type Float%20%28single-precision%29))
  (|CallParentFunction DeltaSeconds))

(event EventPossessed
  (params (NewController :type Controller%20Object%20Reference))
  (|CallParentFunction NewController)
  (Default|Initialize (Variables|Default|GetReviveComponent)))

(fn ConstructionScript
  (|CallParentFunction))

(fn ClearTimer
  (params (Handle :type Timer%20Handle%20Structure))
  (if (Utilities|Time|IsTimerActivebyHandle Handle)
    (Utilities|Time|ClearandInvalidateTimerbyHandle Handle)))
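; Deprecated test player controller for a medic revive system, tracking Normal, Revived, Wounded and Dead states.
; OnRep_MedicalState drives wounded/death screens, revive cleanup and respawning at a player start spawned with the revive actor.
; Use also handles vehicles; for medics it traces for a revive spawner and holds via retriggerable delay and gate before ServerRevive.
; A looping timer refreshes revive-icon team visibility; team changes force Dead, and debug prints remain throughout.
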(event Custom|AddReviveSpawner
  (params (DeathTransform :type Transform) (TeamNum :type Byte))
  ;[1 1 1] Spawn the Revive Actor and Revive Spawn Actor
  (bind _revivetransform (Utilities|CreateReviveSpawner DeathTransform TeamNum)
    (:Exit
      (bind _returnvalue (Game|SpawnActorfromClass "/Script/HDMain.HDPlayerStart" _revivetransform "Undefined" 0 0))
      (Variables|Default|SetReviveStart _returnvalue))))

(event Custom|RevivePlayer
  ;[1 1 1] Helpers
  (Variables|Default|SetMedicalState "NewEnumerator1"))

(event Custom|ServerRevive
  (params (Revive :type BP%20HD%20Revive%20Spawner%20Object%20Reference) (Char :type BP%20HD%20Player%20Character%20Med%20Object%20Reference))
  ;[1 1 1] Trace For Revive Actor
  ;
  ; Check USE Is Held For ReviveHoldTIme
  ;
  ; and Initiate Revive
  (Default|Revive Revive))

(event Custom|InitiateRevive
  ;[1 1 1] Trace For Revive Actor
  ;
  ; Check USE Is Held For ReviveHoldTIme
  ;
  ; and Initiate Revive
  (if (Variables|/MedicalTest/Core/AC_HDReviveCharacter.AC_HDReviveCharacter_C|GetMedic (Variables|/MedicalTest/Core/BP_HDPlayerCharacter_Med.BP_HDPlayerCharacter_Med_C|GetReviveComponent (Variables|Default|GetPChar)))
    (bind _asbp_hdrevive_spawner (Utilities|TraceforReviveActor))
    (Default|StartFillingProgressBar _asbp_hdrevive_spawner)
    (CallFunction|OnHold)
    (Utilities|FlowControl|Gate true) ; enters at Open
    (else
      (Development|PrintString "NotMedic" true true "(R=1.000000,G=0.000000,B=0.019754,A=1.000000)"))))

(event Custom|OnHold
  ;[1 1 1] Trace For Revive Actor
  ;
  ; Check USE Is Held For ReviveHoldTIme
  ;
  ; and Initiate Revive
  (Utilities|FlowControl|RetriggerableDelay (Variables|Default|GetReviveHoldTime))
  (Utilities|FlowControl|Gate true
    (:Exit
      (CallFunction|ServerRevive (stale Custom|InitiateRevive _asbp_hdrevive_spawner) (Variables|Default|GetPChar)))))

(event Custom|OnWounded
  ;[0.9583 1 0.9167] OnRep Medical States: Triggers when Player's medical States changes (Normal, Revivable, Wounded, Death)
  ;;[1 0.2633 0] OnWounded (Player is incapaciatated but Revivable)
  (Development|PrintString "Wounded" true true "(R=1.000000,G=0.402985,B=0.000000,A=1.000000)")
  (Development|PrintString "Wounded" true true "(R=1.000000,G=0.463735,B=0.000000,A=1.000000)")
  (Networking|CanExecuteCosmeticEvents
    (:True
      (CallFunction|WoundedScreenToggle true))))

(event Custom|OnRevived
  ;[0.9583 1 0.9167] OnRep Medical States: Triggers when Player's medical States changes (Normal, Revivable, Wounded, Death)
  ;;[1 0.9253 0] OnRevived(Player is Alive but will become Dead (unrevivable) on Death)
  (Development|PrintString "Revived" true true "(R=1.000000,G=0.809269,B=0.000000,A=1.000000)")
  (Networking|CanExecuteCosmeticEvents
    (:True
      (CallFunction|WoundedScreenToggle false))
    (:False
      (CallFunction|GetReviveKit)
      (Class|GameModeBase|RestartPlayeratPlayerStart (Game|GetGameMode) self (Variables|Default|GetReviveStart))
      (CallFunction|DestroyRevive))))

(event Custom|EnableMedicUI
  ;[1 1 1] Handles Revive Icon UI
  (if (Utilities|Time|IsValidTimerHandle (Variables|Default|GetMedicHandle))
    (Utilities|Time|UnpauseTimerbyHandle (Variables|Default|GetMedicHandle))
    (else
      (bind _returnvalue (Utilities|Time|SetTimerbyEvent (delegate Custom|MedicTimer) 0.3 true))
      (Variables|Default|SetMedicHandle _returnvalue))))

(event Custom|DestroyRevive
  ;[1 1 1] DestroyReviveActor/ReviveStart
  (Utilities|IsValid (Variables|Default|GetRevive)
    (:Is%20Valid
      (Actor|DestroyActor (Variables|Default|GetRevive))
      (Variables|Default|SetRevive 0)
      (Utilities|IsValid (Variables|Default|GetReviveStart)
        (:Is%20Valid
          (Actor|DestroyActor (Variables|Default|GetReviveStart))
          (Variables|Default|SetReviveStart 0))
        (:Is%20Not%20Valid
          (Development|PrintString "DestroyingInvalidReviveStart"))))
    (:Is%20Not%20Valid
      (Development|PrintString "DestroyingInvalidRevive"))))

(event Custom|DisableMedicUI
  ;[1 1 1] Handles Revive Icon UI
  (if (Utilities|Time|IsValidTimerHandle (Variables|Default|GetMedicHandle))
    (Utilities|Time|PauseTimerbyHandle (Variables|Default|GetMedicHandle)))
  (for _array_element (Variables|Default|GetReviveSpawners)
    (Default|HideReviveSpawner _array_element)))

(event Custom|MedicTimer
  ;[1 1 1] Handles Revive Icon UI
  (for _array_element (Variables|Default|GetReviveSpawners)
    (Default|CheckTeamforVisibility _array_element (Variables|Default|GetPChar))))

(event Custom|OnDead
  ;[0.9583 1 0.9167] OnRep Medical States: Triggers when Player's medical States changes (Normal, Revivable, Wounded, Death)
  ;;[1 0 0.02628] OnDead (Player is incapacitated but unable to be revived "DeadDead')
  (Development|PrintString "Dead" true true "(R=1.000000,G=0.011936,B=0.000000,A=1.000000)")
  (Networking|CanExecuteCosmeticEvents
    (:True
      (CallFunction|WoundedScreenToggle false)
      (CallFunction|DeathScreenToggle true))
    (:False
      (CallFunction|DestroyRevive))))

(event Custom|OnNormal
  ;[0.9583 1 0.9167] OnRep Medical States: Triggers when Player's medical States changes (Normal, Revivable, Wounded, Death)
  ;;[0.01576 1 0] OnNormal(Player is Alive and Will Become Wounded On Death)
  (Development|PrintString "Normal" true true "(R=0.086353,G=1.000000,B=0.040309,A=1.000000)")
  (Networking|CanExecuteCosmeticEvents
    (:True
      (CallFunction|DeathScreenToggle false)
      (CallFunction|WoundedScreenToggle false))))

(event Custom|KillPlayer
  ;[1 1 1] Helpers
  (Networking|CanExecuteCosmeticEvents
    (:True
      (Development|PrintString "Killed")
      (CallFunction|ServerKillPlayer))
    (:False
      (Variables|Default|SetMedicalState "NewEnumerator3"))))

(event Custom|ServerKillPlayer
  ;[1 1 1] Helpers
  (Variables|Default|SetMedicalState "NewEnumerator3"))

(event Custom|ReleaseCancel
  ;[1 1 1] Trace For Revive Actor
  ;
  ; Check USE Is Held For ReviveHoldTIme
  ;
  ; and Initiate Revive
  (Utilities|FlowControl|Gate true) ; enters at Close
)

(event EventPlayerTeamNumUpdated
  (params (LastTeamNum :type Byte :default 0) (NewTeamNum :type Byte :default 0))
  ;[1 1 1] SetToDeadOnTeamChange
  (|CallParentFunction LastTeamNum NewTeamNum)
  (if (Utilities|Enum|NotEqual(Enum) (Variables|Default|GetMedicalState) "NewEnumerator3")
    (Variables|Default|SetMedicalState "NewEnumerator3")))

(event EventCharacterDeath
  (params (VictimPawn :type Pawn%20Object%20Reference) (VictimController :type Controller%20Object%20Reference) (KillingDamage :type Float%20%28single-precision%29) (DamageEvent :type Damage%20Event%20Structure%20%28by%20ref%29) (InstigatingPawn :type Pawn%20Object%20Reference) (DamageCauser :type Actor%20Object%20Reference))
  ;[1 1 1] MovedUIHandlingFromDelegateToOnRep
  (bind _asbp_hdhudbase (Utilities|Casting|CastToBP_HDHUDBase (HUD|GetHUD)))
  (Default|ToggleEquipmentUI _asbp_hdhudbase false)
  (bind _asdfbase_character (Utilities|Casting|CastToDFBaseCharacter VictimPawn))
  ;;[1 1 1] Unbind from Character Death event here as the controller will have been detached before the death delegate is broadcasted which would lead to the event being unbound (if unbind is performed in UnpossessPawn()) before it can have a chance to get triggered
  (EventDispatchers|UnbindEventfromOnCharacterDeath _asdfbase_character (EventDispatchers|CreateEvent :!event CharacterDeath)))

(event EventPossessPawn
  (params (NewPawn :type Pawn%20Object%20Reference))
  ;[1 1 1] ResetMedicalStateOnSpawn
  (Variables|Default|SetbInitialSpawn false)
  (switch Utilities|FlowControl|Switch|SwitchonMedicalStateEnum (Variables|Default|GetMedicalState)
    (:NewEnumerator0
      _)
    (:NewEnumerator1
      _)
    (:NewEnumerator2
      (CallFunction|DestroyRevive)
      (Variables|Default|SetMedicalState "NewEnumerator0" :!label _label))
    (:NewEnumerator3
      (goto _label)))
  (bind _asbp_hdplayer_character_med (Utilities|Casting|CastToBP_HDPlayerCharacter_Med NewPawn)
    (:then
      (bind _output_get (Variables|Default|SetPChar _asbp_hdplayer_character_med)))
    (:CastFailed
      _))
  (EventDispatchers|BindEventtoOnCharacterDeath _output_get (EventDispatchers|CreateEvent :!event CharacterDeath)))

(event EventUnpossessPawn
  (params (UnpossessedPawn :type Pawn%20Object%20Reference))
  ;[1 1 1] Handles Revive Icon UI
  (|CallParentFunction UnpossessedPawn)
  (CallFunction|DisableMedicUI))

(event EventBeginPlay
  ;[1 1 1] Handles Revive Icon UI
  (|CallParentFunction)
  (CallFunction|LoadWoundedScreen))

(event EventTick
  (params (DeltaSeconds :type Float%20%28single-precision%29))
  (|CallParentFunction DeltaSeconds)
  (Development|PrintText (Utilities|Text|FormatText "Medical State: {Med}" (Utilities|String|EnumtoString (Variables|Default|GetMedicalState))) true false "(R=0.000000,G=0.660000,B=1.000000,A=1.000000)" 0.0))

(event Input|ActionEvents|InputActionUse
  (params (Key :type Key%20Structure :default "None"))
  (bind _returnvalue (Pawn|GetControlledPawn))
  (bind _returnvalue_2 (Actor|GetComponentbyClass "/Script/ArcVehicles.ArcVehiclePlayerSeatComponent"))
  (bind _returnvalue_3 (Transformation|GetActorLocation _returnvalue))
  (bind _currentseatconfig (Variables|/Script/ArcVehicles.ArcVehiclePlayerSeatComponent|GetCurrentSeatConfig _returnvalue_2))
  ;[1 1 1] ModifiedUseForHoldingToRevive
  (:Pressed
    (bind _asarc_base_vehicle (Utilities|Casting|CastToArcBaseVehicle _returnvalue)
      (:then
        (CallFunction|RequestExitVehicle _asarc_base_vehicle))
      (:CastFailed
        (Utilities|IsValid _returnvalue_2
          (:Is%20Valid
            (if (Class|ArcVehicleBPFunctionLibrary|IsSeatRefValid _currentseatconfig)
              (CallFunction|RequestExitVehicle (Class|ArcVehicleBPFunctionLibrary|GetVehiclefromSeatConfig _currentseatconfig))
              (else
                (bind _asdfbase_player_character (Utilities|Casting|CastToDFBasePlayerCharacter _returnvalue :!label _label)
                  (:then
                    (Class|DFBasePlayerCharacter|Use _asdfbase_player_character)
                    ;;[1 0 0.1606] InitiatedRevive
                    (CallFunction|InitiateRevive))
                  (:CastFailed
                    (bind (_outhit _returnvalue_4) (Collision|LineTraceForObjects _returnvalue_3 (+ _returnvalue_3 (* (Math|Vector|GetForwardVector (Actor|GetComponentbyClass _returnvalue "/Script/Engine.CameraComponent")) 5e+02)) (Utilities|Array|MakeArray "ObjectTypeQuery5") false 0 "ForDuration"))
                    (if _returnvalue_4
                      (bind _asarc_base_vehicle_2 (Utilities|Casting|CastToArcBaseVehicle (.HitActor (Collision|BreakHitResult _outhit))))
                      (Networking|SwitchHasAuthority
                        (:Authority
                          (Class|ArcBaseVehicle|RequestEnterAnySeat _asarc_base_vehicle_2 (Variables|Default|GetPlayerState)))
                        (:Remote
                          (CallFunction|TryGetinVehicle _asarc_base_vehicle_2)))))))))
          (:Is%20Not%20Valid
            (goto _label))))))
  (:Released
    ;;[0.0317 1 0.3512] CancelReviveWhenUseKeyReleased
    (CallFunction|ReleaseCancel)))

(fn ConstructionScript
  (|CallParentFunction))

(fn OnRepMedicalState
  (switch Utilities|FlowControl|Switch|SwitchonMedicalStateEnum (Variables|Default|GetMedicalState)
    (:NewEnumerator0
      (CallFunction|OnNormal))
    (:NewEnumerator1
      (CallFunction|OnRevived))
    (:NewEnumerator2
      (CallFunction|OnWounded))
    (:NewEnumerator3
      (CallFunction|OnDead))))

(fn WoundedScreenToggle
  (params (Show :type Boolean))
  (bind _woundedwidget (Variables|Default|GetWoundedWidget))
  (bind _returnvalue (UserInterface|Viewport|IsinViewport _woundedwidget))
  (Utilities|IsValid _woundedwidget
    (:Is%20Valid
      (if Show
        (if (not _returnvalue)
          (UserInterface|Viewport|AddtoPlayerScreen (Variables|Default|GetWoundedWidget))
          (bind _output_get (Variables|Default|SetbWoundedScreenShown Show :!label _label))
          (if _output_get
            (CallFunction|HideHUD)
            (else
              (CallFunction|ShowHUD))))
        (elif _returnvalue
          (Widget|RemovefromParent (Variables|Default|GetWoundedWidget))
          (goto _label))))))

(fn LoadWoundedScreen
  (Utilities|IsValid (Variables|Default|GetWoundedWidget)
    (:Is%20Not%20Valid
      (bind _returnvalue (UserInterface|CreateWidget "/MedicalTest/Core/UI/Revive/WBP_WoundedScreenRevive.WBP_WoundedScreenRevive_C" self))
      (Variables|Default|SetWoundedWidget _returnvalue))))

(fn GetReviveKit
  (bind _revivestart (Variables|Default|GetReviveStart))
  (bind _returnvalue (Transformation|GetActorLocation _revivestart))
  (bind _outhits (Collision|MultiSphereTraceByChannel _returnvalue _returnvalue 2e+02 "TraceTypeQuery1" false 0 "None"))
  (bind _array_element (Utilities|Array|ForEachLoopwithBreak _outhits :!label _label)
    (:LoopBody
      (if (Utilities|ClassIsChildOf (Utilities|GetClass (|GetHitActor_2_2_2 _array_element)) "/HDCore/Core/BP_HDKitPickupBase.BP_HDKitPickupBase_C")
        (bind _asbp_hdkit_pickup_base (Utilities|Casting|CastToBP_HDKitPickupBase (|GetHitActor_2_2_2 _array_element)))
        (Variables|Default|SetPickupItem _asbp_hdkit_pickup_base)
        (if (== (Utilities|GetClass (|GetHitActor_2_2_2 _array_element)) (Variables|/Script/HDMain.HDKit|GetKitDropPrefabClass (Variables|/Script/HDMain.HDPlayerState|GetSpawnLoadout (CallFunction|GetHDPlayerState))))
          (goto _label Break))))
    (:Completed
      (Variables|/Script/HDMain.HDPlayerComponent|SetStartLoadout (Variables|Default|GetPlayerComponent) "/MedicalTest/Core/Kits/HDKit_Unarmed.HDKit_Unarmed"))))
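; Test player controller that extends the Use input with hold-to-revive alongside vehicle entry and exit.
; Pressing Use exits an occupied Arc vehicle or seat; otherwise a DF character runs its normal Use and starts a revive through ReviveController.
; Other pawns line-trace along the camera's forward direction for a vehicle and request any seat, via server call on clients.
; Releasing Use cancels the revive.
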(event Input|ActionEvents|InputActionUse
  (params (Key :type Key%20Structure :default "None"))
  (bind _returnvalue (Pawn|GetControlledPawn))
  (bind _returnvalue_2 (Transformation|GetActorLocation _returnvalue))
  (bind _returnvalue_3 (Actor|GetComponentbyClass _returnvalue "/Script/ArcVehicles.ArcVehiclePlayerSeatComponent"))
  (bind _currentseatconfig (Variables|/Script/ArcVehicles.ArcVehiclePlayerSeatComponent|GetCurrentSeatConfig _returnvalue_3))
  ;[1 1 1] ModifiedUseForHoldingToRevive
  (:Pressed
    (bind _asarc_base_vehicle (Utilities|Casting|CastToArcBaseVehicle _returnvalue)
      (:then
        (CallFunction|ServerRequestExitVehicle _asarc_base_vehicle))
      (:CastFailed
        (Utilities|IsValid _returnvalue_3
          (:Is%20Valid
            (if (Class|ArcVehicleBPFunctionLibrary|IsSeatRefValid _currentseatconfig)
              (CallFunction|ServerRequestExitVehicle (Class|ArcVehicleBPFunctionLibrary|GetVehiclefromSeatConfig _currentseatconfig))
              (else
                (bind _asdfbase_player_character (Utilities|Casting|CastToDFBasePlayerCharacter _returnvalue :!label _label)
                  (:then
                    (Class|DFBasePlayerCharacter|Use _asdfbase_player_character)
                    ;;[1 0 0.1606] InitiatedRevive
                    (Default|InitiateRevive (Variables|Default|GetReviveController)) ; Can't really integrate this with Use because revive is supposed to be held. \nOnce epipen is implemented, probably wont need the 2nd trace.
                  )
                  (:CastFailed
                    (bind (_outhit _returnvalue_4) (Collision|LineTraceForObjects _returnvalue_2 (+ _returnvalue_2 (* (Math|Vector|GetForwardVector (Actor|GetComponentbyClass _returnvalue "/Script/Engine.CameraComponent")) 5e+02)) (Utilities|Array|MakeArray "ObjectTypeQuery5") false 0 "ForDuration"))
                    (if _returnvalue_4
                      (bind _asarc_base_vehicle_2 (Utilities|Casting|CastToArcBaseVehicle (.HitActor (Collision|BreakHitResult _outhit))))
                      (Networking|SwitchHasAuthority
                        (:Authority
                          (Class|ArcBaseVehicle|RequestEnterAnySeat _asarc_base_vehicle_2 (Variables|Default|GetPlayerState)))
                        (:Remote
                          (CallFunction|ServerTryGetinVehicle _asarc_base_vehicle_2)))))))))
          (:Is%20Not%20Valid
            (goto _label))))))
  (:Released
    ;;[0.0317 1 0.3512] CancelReviveWhenUseKeyReleased
    (Default|ReleaseCancel (Variables|Default|GetReviveController)) ; Cancels Revive when Use released
  ))

(fn ConstructionScript
  (|CallParentFunction))

(fn GetReviveController
  (return (Variables|Default|GetReviveController)))
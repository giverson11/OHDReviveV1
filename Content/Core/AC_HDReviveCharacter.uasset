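; Character component for a revive and medic system, working through the controller's AC_HDReviveController, which holds medical state.
; A Normal death becomes Wounded and adds a revive spawner, while dying when Revived means Dead.
; Initializing as Revived re-equips the kit at low health, prones the player and starts a timer to Normal, which full healing also triggers.
; It scans inventory for a medbox to set medic status and UI, routed between server and client by authority.
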(event Custom|Initialize
  (bind _playerchar (Variables|Default|GetPlayerChar))
  (bind _playerchar_2 (Variables|Default|GetPlayerChar))
  (bind _returnvalue (Pawn|GetController _playerchar_2))
  (bind _returnvalue_2 (Actor|GetComponentbyClass _returnvalue "/MedicalTest/Core/AC_HDReviveController.AC_HDReviveController_C"))
  ;[1 1 1] Pickup Nearby Kit and Prone if Revived then Check if Medic
  ;
  ; Otherwise just Check if Medic if Spawned Normally
  (Development|PrintString "Initialized" true false "(R=0.000000,G=1.000000,B=0.032413,A=1.000000)")
  (Utilities|IsValid _returnvalue_2
    (:Is%20Valid
      (Variables|Default|SetReviveController _returnvalue_2)
      (EventDispatchers|AssignOnHealthChanged _playerchar (delegate Custom|ClearRevivedOnFullHeal))
      (EventDispatchers|AssignOnCharacterDeath _playerchar (delegate Custom|OnDeath))
      (if (Utilities|CheckMedicalState "NewEnumerator1")
        (Utilities|OwnerHasAuthority
          (:Authority
            (CallFunction|EquipKit)
            (CallFunction|CheckifMedic)
            (CallFunction|ClientonRevive))
          (:Remote
            (CallFunction|ServerEquipKit)))
        (else
          (Utilities|OwnerHasAuthority
            (:Authority
              (Variables|Default|SetCanCheckMedic true)
              (CallFunction|CheckifMedic))
            (:Remote
              (CallFunction|ServerCheckifMedic))))))))

(event Custom|ServerEquipKit
  ;[1 1 1] Picks up nearby kit on Revive
  ;
  ; Sets a timer that sets Medical State to Normal after elapsed time.
  (CallFunction|EquipKit))

(event Custom|ServerCheckIfMedic
  ;[1 1 1] CheckIfMedic (Fairly Inefficient and Sketchy Solution)
  ;;[1 0.6858 0.02494] CheckIfMedicOnKitPickup
  (Variables|Default|SetCanCheckMedic true)
  (CallFunction|CheckifMedic))

(event Custom|ClientOnRevive
  ;[1 1 1] CheckIfMedic (Fairly Inefficient and Sketchy Solution)
  ;;[1 0.6858 0.02494] CheckIfMedicOnKitPickup
  (Utilities|FlowControl|Delay 0.01)
  (Class|DFBaseCharacter|ProneToggle (Variables|Default|GetPlayerChar))
  (Default|GenericDamageFeedback (Variables|Default|GetPlayerChar)))

(event Custom|EquipKit
  (bind _revivecontroller (Variables|Default|GetReviveController))
  (bind _pickupitem (Variables|/MedicalTest/Core/AC_HDReviveController.AC_HDReviveController_C|GetPickupItem _revivecontroller))
  ;[1 1 1] Picks up nearby kit on Revive
  ;
  ; Sets a timer that sets Medical State to Normal after elapsed time.
  (Utilities|FlowControl|Delay 0.01)
  (Variables|Default|SetCanCheckMedic true)
  (if (Utilities|CheckMedicalState "NewEnumerator1")
    (Utilities|IsValid _pickupitem
      (:Is%20Valid
        (Class|HDPlayerCharacter|OnPickupKit (Variables|Default|GetPlayerChar) _pickupitem))
      (:Is%20Not%20Valid
        _))
    (Variables|/Script/DonkehFramework.DFBaseCharacter|SetHealth (Variables|Default|GetPlayerChar) 2e+01)
    (bind _returnvalue (Utilities|Time|SetTimerbyEvent (delegate Custom|InstaDeathCounter) (Variables|Default|GetTimeToClearInstaDeath)))
    (Variables|Default|SetDeadDeadHandle _returnvalue)))

(event Custom|ClearRevivedOnFullHeal
  (params (Character :type DF%20Base%20Character%20Object%20Reference) (NewHealthTotal :type Float%20%28single-precision%29) (PrevHealthTotal :type Float%20%28single-precision%29))
  ;[1 1 1] Pickup Nearby Kit and Prone if Revived then Check if Medic
  ;
  ; Otherwise just Check if Medic if Spawned Normally
  ;;[1 0.3193 0] If Health Reaches Full After Being Recently Player is Revivable On Death
  (if (and (== NewHealthTotal 1e+02) (Utilities|CheckMedicalState "NewEnumerator1"))
    (Utilities|SetMedicalState "NewEnumerator0")
    (CallFunction|ClearTimer (Variables|Default|GetDeadDeadHandle))))

(event Custom|InstaDeathCounter
  ;[1 1 1] Picks up nearby kit on Revive
  ;
  ; Sets a timer that sets Medical State to Normal after elapsed time.
  (Utilities|SetMedicalState "NewEnumerator0")
  (Utilities|Time|ClearandInvalidateTimerbyHandle (Variables|Default|GetDeadDeadHandle)))

(event Custom|SetMedic
  (params (Medic :type Boolean))
  ;[1 1 1] CheckIfMedic (Fairly Inefficient and Sketchy Solution)
  ;;[1 0 0.7758] Checks if Medic and displays or hides medic UI (depending on if medical kit is in inventory)
  ;;
  ;; CanMedicCheck is there to prevent CheckIfMedicOnKitPickup from firing on spawn as it is triggered twice for some reason and triggers before some begin play variables are initialized
  (Variables|Default|SetMedic Medic))

(event Custom|OnDeath
  (params (VictimPawn :type Pawn%20Object%20Reference) (VictimController :type Controller%20Object%20Reference) (KillingDamage :type Float%20%28single-precision%29) (DamageEvent :type Damage%20Event%20Structure%20%28by%20ref%29) (InstigatingPawn :type Pawn%20Object%20Reference) (DamageCauser :type Actor%20Object%20Reference))
  (CallFunction|ClearTimer (Variables|Default|GetDeadDeadHandle))
  (Utilities|OwnerHasAuthority
    (:Authority
      (switch Utilities|FlowControl|Switch|SwitchonMedicalStateEnum (Variables|/MedicalTest/Core/AC_HDReviveController.AC_HDReviveController_C|GetMedicalState (Variables|Default|GetReviveController))
        (:NewEnumerator0
          (Utilities|SetMedicalState "NewEnumerator2")
          (Default|AddReviveSpawner (Variables|Default|GetReviveController) (Transformation|GetActorTransform (Variables|Default|GetPlayerChar)) (Class|DFBlueprintFunctions|GetTeamNum (Variables|Default|GetPlayerChar))))
        (:NewEnumerator1
          (Utilities|SetMedicalState "NewEnumerator3"))))))

(event Custom|ClientShowMedicUI
  (params (Enabled :type Boolean))
  ;[1 1 1] CheckIfMedic (Fairly Inefficient and Sketchy Solution)
  ;;[1 0 0.7758] Checks if Medic and displays or hides medic UI (depending on if medical kit is in inventory)
  ;;
  ;; CanMedicCheck is there to prevent CheckIfMedicOnKitPickup from firing on spawn as it is triggered twice for some reason and triggers before some begin play variables are initialized
  (Utilities|ShowMedicUI Enabled))

(event Custom|ServerSetMedic
  (params (Medic :type Boolean))
  ;[1 1 1] CheckIfMedic (Fairly Inefficient and Sketchy Solution)
  ;;[1 0 0.7758] Checks if Medic and displays or hides medic UI (depending on if medical kit is in inventory)
  ;;
  ;; CanMedicCheck is there to prevent CheckIfMedicOnKitPickup from firing on spawn as it is triggered twice for some reason and triggers before some begin play variables are initialized
  (CallFunction|SetMedic Medic))

(event Custom|CheckIfMedic
  ;[1 1 1] CheckIfMedic (Fairly Inefficient and Sketchy Solution)
  ;;[1 0 0.7758] Checks if Medic and displays or hides medic UI (depending on if medical kit is in inventory)
  ;;
  ;; CanMedicCheck is there to prevent CheckIfMedicOnKitPickup from firing on spawn as it is triggered twice for some reason and triggers before some begin play variables are initialized
  (if (Variables|Default|GetCanCheckMedic)
    (Development|PrintString "Checking" true true "(R=1.000000,G=0.993306,B=0.000000,A=1.000000)" 8.0)
    (Variables|Default|SetIsMedic false)
    (bind _array_element (Utilities|Array|ForEachLoopwithBreak (Variables|/Script/DonkehFramework.DFInventoryComponent|GetItems (Variables|/Script/DonkehFramework.DFBaseCharacter|GetInventory (Variables|Default|GetPlayerChar))) :!label _label)
      (:LoopBody
        (bind _ismedbox (CallFunction|MedboxCheck _array_element))
        (if _ismedbox
          (Variables|Default|SetIsMedic true)
          (Utilities|OwnerHasAuthority
            (:Authority
              (CallFunction|SetMedic true)
              (CallFunction|ClientShowMedicUI true))
            (:Remote
              (CallFunction|ServerSetMedic true)
              (Utilities|ShowMedicUI true
                (:Exit
                  _))))
          (Development|PrintString "MedicPicked" true true "(R=1.000000,G=0.000000,B=0.943358,A=1.000000)")
          (goto _label Break)))
      (:Completed
        (if (not (Variables|Default|GetIsMedic))
          (Development|PrintString "MedicNotPicked" true true "(R=1.000000,G=0.000000,B=0.095176,A=1.000000)")
          (Utilities|OwnerHasAuthority
            (:Authority
              (CallFunction|SetMedic false)
              (CallFunction|ClientShowMedicUI false))
            (:Remote
              (CallFunction|ServerSetMedic false)
              (Utilities|ShowMedicUI false))))))))

(event EventTick
  (params (DeltaSeconds :type Float%20%28single-precision%29)))

(event EventBeginPlay
  (bind _asbp_hdplayer_character_base (Utilities|Casting|CastToBP_HDPlayerCharacterBase (Components|GetOwner))
    (:then
      (Variables|Default|SetPlayerChar _asbp_hdplayer_character_base)
      (Development|PrintString "ReviveStarting" true true "(R=1.000000,G=0.970537,B=0.992634,A=1.000000)"))
    (:CastFailed
      (Components|Activation|Deactivate)
      (Development|PrintString "CharacterCastFailed" true true "(R=1.000000,G=0.983531,B=0.962442,A=1.000000)"))))
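; Revive point actor for a player, letting a same-team medic revive them through the stored owning controller.
; On clients it registers with the local player controller's ReviveSpawners array, and on destruction deregisters and destroys the stored player character.
; Team and distance checks toggle the widget icon, while sphere overlaps drive its proximity prompt and a targeting event starts its progress fill.
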(event OnComponentBeginOverlap(UISphere)
  (params (OverlappedComponent :type Primitive%20Component%20Object%20Reference) (OtherActor :type Actor%20Object%20Reference) (OtherComp :type Primitive%20Component%20Object%20Reference) (OtherBodyIndex :type Integer) (bFromSweep :type Boolean) (SweepResult :type Hit%20Result%20Structure%20%28by%20ref%29))
  ;[1 1 1] Displays "Press F to Revive" When Player is Close
  (bind _asbp_hdplayer_character_base (Utilities|Casting|CastToBP_HDPlayerCharacterBase OtherActor))
  (if (Class|DFBlueprintFunctions|IsLocallyPlayerControlled _asbp_hdplayer_character_base)
    (Default|OnOverlap (Variables|Default|GetIcon))))

(event OnComponentEndOverlap(UISphere)
  (params (OverlappedComponent :type Primitive%20Component%20Object%20Reference) (OtherActor :type Actor%20Object%20Reference) (OtherComp :type Primitive%20Component%20Object%20Reference) (OtherBodyIndex :type Integer))
  ;[1 1 1] Displays "Press F to Revive" When Player is Close
  (bind _asbp_hdplayer_character_base (Utilities|Casting|CastToBP_HDPlayerCharacterBase OtherActor))
  (if (Class|DFBlueprintFunctions|IsLocallyPlayerControlled _asbp_hdplayer_character_base)
    (Default|OffOverlap (Variables|Default|GetIcon))))

(event Custom|HideReviveSpawner
  ;[1 1 1] ChecksWhenToDisplayReviveIcon
  (Development|SetHiddeninGame (Variables|Default|GetReviveWidget) true false)
  (Variables|Default|SetDeactivateWidget true))

(event Custom|SetupReviveSpawner
  (params (MedController :type BP%20HD%20Player%20Controller%20Med%20Test%20Object%20Reference) (Team :type Byte))
  ;[1 1 1] Helper
  (bind _output_get (Variables|Default|SetController MedController))
  (Variables|Default|SetTeam Team)
  (Variables|Default|SetChar (Variables|/MedicalTest/Core/BP_HDPlayerController_MedTest.BP_HDPlayerController_MedTest_C|GetPChar _output_get)))

(event Custom|Revive
  (params (Instigator :type BP%20HD%20Player%20Character%20Med%20Object%20Reference))
  (bind _returnvalue (Class|DFBlueprintFunctions|GetTeamNum Instigator))
  (bind _medic (Variables|/MedicalTest/Core/BP_HDPlayerCharacter_Med.BP_HDPlayerCharacter_Med_C|GetMedic Instigator))
  (bind _team (Variables|Default|GetTeam))
  (bind _returnvalue_2 (== _returnvalue _team))
  ;[1 1 1] Checks if Player is Medic and Same Team
  ;
  ; Then Revives
  (if (and _medic _returnvalue_2)
    (Default|RevivePlayer (Variables|Default|GetController))
    (else
      (Development|PrintText (Utilities|Text|FormatText "Can't Revive:  
Medic?: {MED}  
TEAM?: {T}" (Utilities|String|ToString(Boolean) _medic) (Utilities|String|ToString(Boolean) _returnvalue_2)) true true "(R=1.000000,G=0.000000,B=0.014146,A=1.000000)"))))

(event Custom|CheckTeamForVisibility
  (params (Character :type BP%20HD%20Player%20Character%20Base%20Object%20Reference))
  (bind _self self)
  (bind _teamnum (Variables|/Script/DonkehFramework.DFBaseCharacter|GetTeamNum Character))
  (bind _team (Variables|Default|GetTeam))
  (bind _reviveuidistance (Variables|Default|GetReviveUIDistance))
  (bind _returnvalue (!= _teamnum _team))
  (bind _returnvalue_2 (Transformation|GetDistanceTo Character _self))
  (bind _returnvalue_3 (> _returnvalue_2 _reviveuidistance))
  (bind _returnvalue_4 (or _returnvalue_3 _returnvalue))
  ;[1 1 1] ChecksWhenToDisplayReviveIcon
  (Development|SetHiddeninGame (Variables|Default|GetReviveWidget) _returnvalue_4 false)
  (Variables|Default|SetDeactivateWidget _returnvalue_4))

(event Custom|StartFillingProgressBar
  ;[1 1 1] StartsFillingProgressBarOnReviveIcon
  (if (not (Variables|Default|GetDeactivateWidget))
    (Default|SpawnerTargeted (Variables|Default|GetIcon))))

(event EventBeginPlay
  (bind _aswbp_revive_icon (Utilities|Casting|CastToWBP_ReviveIcon (UserInterface|GetUserWidgetObject (Variables|Default|GetReviveWidget))))
  (Variables|Default|SetIcon _aswbp_revive_icon)
  (Variables|Default|SetDeactivateWidget false)
  (Networking|CanExecuteCosmeticEvents
    (:True
      (bind _asbp_hdplayer_controller_med_test (Utilities|Casting|CastToBP_HDPlayerController_MedTest (Widget|GetOwningPlayer (Variables|Default|GetIcon))))
      (Development|PrintString "SpawnerAdded")
      ;[1 1 1] Adds/Removes ReviveSpawnerToControllerArray and destroys body
      (bind _output_get (Variables|Default|SetLocalController _asbp_hdplayer_controller_med_test))
      (Utilities|Array|Add (Variables|/MedicalTest/Core/BP_HDPlayerController_MedTest.BP_HDPlayerController_MedTest_C|GetReviveSpawners _output_get) self))))

(event EventDestroyed
  (bind _char (Variables|Default|GetChar))
  ;[1 1 1] Adds/Removes ReviveSpawnerToControllerArray and destroys body
  (|CallParentFunction)
  (Networking|CanExecuteCosmeticEvents
    (:True
      (Utilities|Array|RemoveItem (Variables|/MedicalTest/Core/BP_HDPlayerController_MedTest.BP_HDPlayerController_MedTest_C|GetReviveSpawners (Variables|Default|GetLocalController)) self)
      (Utilities|IsValid _char
        (:Is%20Valid
          (Actor|DestroyActor _char))))))

(fn ConstructionScript)

(fn EventGetTeamNum
  (return 0))